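; BP_Rail is an interactable rail that carries the player along its spline when they overlap it.
; On overlap it stores the player, disables their movement and plays the Movement timeline from the start, with play rate set from PlayLength at BeginPlay.
; Each update moves the player to the matching distance along the spline.
; When it finishes, movement is re-enabled and the rail frees up for reuse.
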(event Custom|StartMovement
  (bind _spline (Variables|Default|GetSpline))
  ;[1 1 1] Spline Movement
  (bind _percentcompleted (Timeline|Movement PlayFromStart)
    (:Update
      (Transformation|SetActorLocationAndRotation (Variables|Default|GetPlayer) (Spline|GetLocationatDistanceAlongSpline _spline (* (Spline|GetSplineLength _spline) _percentcompleted) "World")))
    (:Finished
      (Default|EnableMovement (Variables|Default|GetPlayer))
      (Variables|Default|SetPlayer 0))))

(event EventBeginPlay
  ;[1 1 1] Set Play Rate
  (Components|Timeline|SetPlayRate (Variables|Default|GetMovement) (/ 1.0 (Variables|SplineMovement|GetPlayLength))))

(event Collision|EventActorBeginOverlap
  (params (OtherActor :type Actor%20Object%20Reference))
  ;[1 1 1] Handle Overlap
  (Utilities|IsValid (Variables|Default|GetPlayer)
    (:Is%20Not%20Valid
      (bind _asbp_player (Utilities|Casting|CastToBP_Player OtherActor))
      (bind _output_get (Variables|Default|SetPlayer _asbp_player))
      (Default|DisableMovement _output_get)
      (CallFunction|StartMovement))))

(fn ConstructionScript)