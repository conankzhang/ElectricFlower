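; InfiniumTower is a tower Blueprint with health that reacts to a TakeDamage event.
; Each hit subtracts damage from Health, spawns an attached burst effect above the Base and destroys it after a short delay.
; The death check runs only when that effect is no longer valid after the delay, and just prints a message at zero or lower Health.
; GetPoints is a stub returning zero.
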(event EventBeginPlay)

(event Collision|EventActorBeginOverlap
  (params (OtherActor :type Actor%20Object%20Reference)))

(event EventTick
  (params (DeltaSeconds :type Float%20%28single-precision%29)))

(event EventTakeDamage
  (params (i_Damage :type Integer) (Impulse :type Vector :default "0, 0, 0"))
  (bind _output_get (Variables|Default|SetHealth (- (Variables|Default|GetHealth) i_Damage)))
  (bind _returnvalue (Effects|SpawnEmitterAttached "/Game/_VFX/Particles/P_Burst_VFX.P_Burst_VFX" 0 "None" (Math|Vector|MakeVector 0.0 0.0 (+ (.z (Transformation|GetWorldLocation (Variables|Default|Getbase))) 1e+02)) "0, 0, 0" "3.500000,3.500000,3.500000"))
  (Utilities|FlowControl|Delay 2.0)
  (if (Utilities|IsValid _returnvalue)
    (Components|DestroyComponent _returnvalue)
    (else
      ;[1 1 1] Check for Tower Death
      (Math|Integer|CompareInt _output_get
        (:==
          _)
        (:<
          _))
      (Development|PrintString "InfiniumTower down. Health <= 0"))))

(fn ConstructionScript)

(fn GetPoints
  (return 0))