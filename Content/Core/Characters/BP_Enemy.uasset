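; Enemy character that reacts to spotting the player, switching between a calm and a scary look.
; PawnSensing stores the seen player, swaps meshes and turns the spotlight red; OnLostPawn clears it, restores the calm look and flags ReturnHome.
; AddMovementInputCustom faces the given direction and applies movement scaled by PursuitSpeed.
; Kill spawns a particle effect, sets the LightArray lights' intensity and destroys the enemy.
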(event OnSeePawn(PawnSensing)
  (params (Pawn :type Pawn%20Object%20Reference))
  (bind _asbp_player (Utilities|Casting|CastToBP_Player Pawn))
  (Variables|Default|SetPlayer _asbp_player)
  (Rendering|SetVisibility (Variables|Default|GetCalmMesh) false false)
  (Rendering|SetVisibility (Variables|Default|GetScaryMesh) true false)
  (Rendering|Components|Light|SetLightColor (Variables|Default|GetSpotLight) "(R=1.000000,G=0.000000,B=0.000000,A=1.000000)" true))

(event Custom|On%20Lost%20Pawn
  (Variables|Default|SetbReturnHome true)
  (Variables|Default|SetPlayer 0)
  (Rendering|SetVisibility (Variables|Default|GetCalmMesh) true false)
  (Rendering|SetVisibility (Variables|Default|GetScaryMesh) false false)
  (Rendering|Components|Light|SetLightColor (Variables|Default|GetSpotLight) "(R=1.000000,G=1.000000,B=1.000000,A=1.000000)" true))

(event Custom|Kill
  (Effects|SpawnEmitteratLocation "/Game/VFX/P_LevelUp_VFX.P_LevelUp_VFX" (Transformation|GetActorLocation))
  (for _array_element (Variables|Default|GetLightArray)
    (Rendering|Components|Light|SetIntensity (Variables|/Script/Engine.Light|GetLightComponent _array_element) 2.5e+03))
  (Actor|DestroyActor))

(event EventAddMovementInputCustom
  (params (WorldDirection :type Vector :default "0, 0, 0") (ScaleValue :type Float%20%28single-precision%29))
  ;[1 1 1] Pursuit Movement
  (Transformation|SetActorRotation (|GetRotation WorldDirection))
  (Pawn|Input|AddMovementInput WorldDirection (* ScaleValue (Variables|Default|GetPursuitSpeed)) false))

(fn ConstructionScript)

(fn GetPlayer
  (return (Variables|Default|GetPlayer)))