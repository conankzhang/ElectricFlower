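; Player pawn that flies freely with a FloatingPawnMovement component, steered by controller yaw/pitch and camera-relative forward and strafe input plus vertical input.
; An overlap sphere tracks the BP_Enemy in range, and Attack kills it and triggers Grow.
; Grow briefly boosts the firefly, center-light and heat parameters of the electric-flower particle effect, then restores the defaults set on BeginPlay.
; EnableMovement and DisableMovement gate movement input, with enabling also zeroing velocity.
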(event OnComponentBeginOverlap(Sphere)
  (params (OverlappedComponent :type Primitive%20Component%20Object%20Reference) (OtherActor :type Actor%20Object%20Reference) (OtherComp :type Primitive%20Component%20Object%20Reference) (OtherBodyIndex :type Integer) (bFromSweep :type Boolean) (SweepResult :type Hit%20Result%20Structure%20%28by%20ref%29))
  (bind _asbp_enemy (Utilities|Casting|CastToBP_Enemy OtherActor))
  (Variables|Default|SetEnemyToKill _asbp_enemy))

(event OnComponentEndOverlap(Sphere)
  (params (OverlappedComponent :type Primitive%20Component%20Object%20Reference) (OtherActor :type Actor%20Object%20Reference) (OtherComp :type Primitive%20Component%20Object%20Reference) (OtherBodyIndex :type Integer))
  (Utilities|Casting|CastToBP_Enemy OtherActor)
  (Variables|Default|SetEnemyToKill 0))

(event Custom|Grow
  (bind _p_elecflower_vfx_bp_control (Variables|Default|GetP_ElecFlower_VFX_BP_control))
  (Effects|Components|ParticleSystem|SetFloatParameter _p_elecflower_vfx_bp_control "DiscardFireflySpawnRate" 1e+02)
  (Effects|Components|ParticleSystem|SetFloatParameter _p_elecflower_vfx_bp_control "SurroundFireflySpawnRate" 1e+02)
  (Effects|Components|ParticleSystem|SetFloatParameter _p_elecflower_vfx_bp_control "FireFlyVelocity" -3.5)
  (Effects|Components|ParticleSystem|SetVectorParameter _p_elecflower_vfx_bp_control "CenterLightSize" "150.000000,150.000000,150.000000")
  (Effects|Components|ParticleSystem|SetVectorParameter _p_elecflower_vfx_bp_control "CenterLightIntense" "300.000000,600.000000,300.000000")
  (Effects|Components|ParticleSystem|SetVectorParameter _p_elecflower_vfx_bp_control "HeatRange" "300.000000,300.000000,300.000000")
  (Utilities|FlowControl|Delay 2.0)
  (Effects|Components|ParticleSystem|SetFloatParameter _p_elecflower_vfx_bp_control "SurroundFireflySpawnRate" 2.0)
  (Effects|Components|ParticleSystem|SetFloatParameter _p_elecflower_vfx_bp_control "FireFlyVelocity" -1.0)
  (Effects|Components|ParticleSystem|SetFloatParameter _p_elecflower_vfx_bp_control "DiscardFireflySpawnRate" 5.0)
  (Effects|Components|ParticleSystem|SetVectorParameter _p_elecflower_vfx_bp_control "CenterLightIntense" "75.000000,150.000000,75.000000")
  (Effects|Components|ParticleSystem|SetVectorParameter _p_elecflower_vfx_bp_control "CenterLightSize" "100.000000,100.000000,100.000000")
  (Effects|Components|ParticleSystem|SetVectorParameter _p_elecflower_vfx_bp_control "HeatRange" "200.000000,200.000000,200.000000"))

(event Custom|Enable%20Movement
  ;[1 1 1] Input Enable/Disable
  (Variables|Default|SetbIsMovementEnabled true)
  (Variables|/Script/Engine.MovementComponent|SetVelocity (Variables|Default|GetFloatingPawnMovement) "0, 0, 0"))

(event Custom|Disable%20Movement
  ;[1 1 1] Input Enable/Disable
  (Variables|Default|SetbIsMovementEnabled false))

(event EventBeginPlay
  (bind _p_elecflower_vfx_bp_control (Variables|Default|GetP_ElecFlower_VFX_BP_control))
  (Effects|Components|ParticleSystem|SetFloatParameter _p_elecflower_vfx_bp_control "DiscardFireflySpawnRate" 5.0)
  (Effects|Components|ParticleSystem|SetFloatParameter _p_elecflower_vfx_bp_control "SurroundFireflySpawnRate" 2.0)
  (Effects|Components|ParticleSystem|SetVectorParameter _p_elecflower_vfx_bp_control "CenterLightIntense" "75.000000,150.000000,75.000000")
  (Effects|Components|ParticleSystem|SetVectorParameter _p_elecflower_vfx_bp_control "HeatRange" "200.000000,200.000000,200.000000")
  (Effects|Components|ParticleSystem|SetFloatParameter _p_elecflower_vfx_bp_control "FireFlyVelocity" -1.0)
  (Effects|Components|ParticleSystem|SetVectorParameter _p_elecflower_vfx_bp_control "CenterLightSize" "100.000000,100.000000,100.000000"))

(event Input|ActionEvents|InputActionAttack
  (params (Key :type Key%20Structure))
  (bind _enemytokill (Variables|Default|GetEnemyToKill))
  (:Pressed
    (Utilities|IsValid _enemytokill
      (:Is%20Valid
        (Default|Kill _enemytokill)
        (CallFunction|Grow)))))

(event Input|AxisEvents|InputAxisYaw
  (params (AxisValue :type Float%20%28single-precision%29))
  ;[1 1 1] Camera Movement
  (Pawn|Input|AddControllerYawInput AxisValue))

(event Input|AxisEvents|InputAxisPitch
  (params (AxisValue :type Float%20%28single-precision%29))
  ;[1 1 1] Camera Movement
  (Pawn|Input|AddControllerPitchInput AxisValue))

(event Input|AxisEvents|InputAxisVertical
  (params (AxisValue :type Float%20%28single-precision%29))
  ;[1 1 1] Vertical Movement
  (if (Variables|Default|GetbIsMovementEnabled)
    (Class|PawnMovementComponent|AddInputVector (Variables|Default|GetFloatingPawnMovement) (Math|Vector|MakeVector 0.0 0.0 AxisValue) false)))

(event Input|AxisEvents|InputAxisLateral
  (params (AxisValue :type Float%20%28single-precision%29))
  ;[1 1 1] Lateral Movement
  (if (Variables|Default|GetbIsMovementEnabled)
    (Class|PawnMovementComponent|AddInputVector (Variables|Default|GetFloatingPawnMovement) (* (Math|Vector|GetRightVector (Variables|Default|GetCamera)) AxisValue) true)))

(event Input|AxisEvents|InputAxisLongitudinal
  (params (AxisValue :type Float%20%28single-precision%29))
  ;[1 1 1] Longitudinal Movement
  (if (Variables|Default|GetbIsMovementEnabled)
    (Class|PawnMovementComponent|AddInputVector (Variables|Default|GetFloatingPawnMovement) (* (Math|Vector|GetForwardVector (Variables|Default|GetCamera)) AxisValue) false)))

(fn ConstructionScript)