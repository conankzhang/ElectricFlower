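; BP_EnemyRail is a patrol rail that moves an assigned enemy along a spline in a repeating loop.
; A timeline scaled by PlayLength drives position and rotation by distance along the spline.
; Updates skip moving the enemy while it has a Player or is returning home.
; The rail's location serves as the enemy's home, and Tick restarts the patrol from the beginning once a returning enemy without a Player gets near it.
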(event Custom|StartMovement
  (bind _spline (Variables|Default|GetSpline))
  (bind _enemy (Variables|Default|GetEnemy))
  ;[1 1 1] Spline Movement
  (bind _percentcompleted (Timeline|Movement PlayFromStart)
    (:Update
      (Utilities|IsValid _enemy
        (:Is%20Valid
          (if (and (not (Utilities|IsValid (Variables|/Game/Core/Characters/BP_Enemy.BP_Enemy_C|GetPlayer _enemy))) (not (Variables|/Game/Core/Characters/BP_Enemy.BP_Enemy_C|GetbReturnHome (Variables|Default|GetEnemy))))
            (Transformation|SetActorLocationAndRotation (Variables|Default|GetEnemy) (Spline|GetLocationatDistanceAlongSpline _spline (* (Spline|GetSplineLength _spline) _percentcompleted) "World") (Spline|GetRotationatDistanceAlongSpline _spline (* (Spline|GetSplineLength _spline) _percentcompleted) "World"))))))
    (:Finished
      (CallFunction|StartMovement))))

(event EventTick
  (params (DeltaSeconds :type Float%20%28single-precision%29))
  (bind _enemy (Variables|Default|GetEnemy))
  (Utilities|IsValid (Variables|Default|GetEnemy)
    (:Is%20Valid
      (if (Math|Boolean|ANDBoolean (Math|Vector|Equal(Vector) (Transformation|GetActorLocation (Variables|Default|GetEnemy)) (Transformation|GetActorLocation) 2e+02) (Variables|/Game/Core/Characters/BP_Enemy.BP_Enemy_C|GetbReturnHome _enemy) (not (Utilities|IsValid (Variables|/Game/Core/Characters/BP_Enemy.BP_Enemy_C|GetPlayer _enemy))))
        (Variables|/Game/Core/Characters/BP_Enemy.BP_Enemy_C|SetbReturnHome (Variables|Default|GetEnemy) false)
        (CallFunction|StartMovement)))))

(event EventBeginPlay
  ;[1 1 1] Set Play Rate
  (Components|Timeline|SetPlayRate (Variables|Default|GetMovement) (/ 1.0 (Variables|SplineMovement|GetPlayLength)))
  (Utilities|IsValid (Variables|Default|GetEnemy)
    (:Is%20Valid
      (Variables|/Game/Core/Characters/BP_Enemy.BP_Enemy_C|SetHomeLocation (Variables|Default|GetEnemy) (Transformation|GetActorLocation))
      (CallFunction|StartMovement))))

(fn ConstructionScript)