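; Lamp post Blueprint that sets its spot light's intensity and removes its particle effect when an actor overlaps it.
; The overlap event applies a fixed intensity to the SpotLight and destroys the ParticleSystem component.
; Tick has a brightening branch gated on WasTouched, but the logic that sets that flag is disconnected and never runs.
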(event EventBeginPlay)

(event EventTick
  (params (DeltaSeconds :type Float%20%28single-precision%29))
  (if (Variables|Default|GetwasTouched)
    (Rendering|Components|Light|SetIntensity (Variables|Default|GetSpotLight) (+ (Variables|Default|Getintensity) 5e+01))
    (Components|DestroyComponent (Variables|Default|GetParticleSystem))))

(event Collision|EventActorBeginOverlap
  (params (OtherActor :type Actor%20Object%20Reference))
  (Rendering|Components|Light|SetIntensity (Variables|Default|GetSpotLight) 5e+02)
  (Components|DestroyComponent (Variables|Default|GetParticleSystem)))

(fn ConstructionScript)